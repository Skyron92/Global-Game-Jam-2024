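; BP_AMB is an ambient sound Blueprint built around five phase loops.
; On BeginPlay it spawns all five loops at once as 2D sounds and stores each audio component in its own phase variable.
; Tick instantly sets only Phase 0's volume to zero through a hardcoded branch with identical sides, so no switching between phases is implemented.
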(event EventBeginPlay
  (Utilities|FlowControl|Sequence
    (:then_0
      (bind _returnvalue (Audio|SpawnSound2D "/Game/Sound/WAV/AMB_LP_Phase0_V01.AMB_LP_Phase0_V01" 1.0 1.0 0.0 0))
      (Variables|Default|SetPhase0 _returnvalue))
    (:then_1
      (bind _returnvalue_2 (Audio|SpawnSound2D "/Game/Sound/WAV/AMB_LP_Phase1_V01.AMB_LP_Phase1_V01" 1.0 1.0 0.0 0))
      (Variables|Default|SetPhase1 _returnvalue_2))
    (:then_2
      (bind _returnvalue_3 (Audio|SpawnSound2D "/Game/Sound/WAV/AMB_LP_Phase2_V01.AMB_LP_Phase2_V01" 1.0 1.0 0.0 0))
      (Variables|Default|SetPhase2 _returnvalue_3))
    (:then_3
      (bind _returnvalue_4 (Audio|SpawnSound2D "/Game/Sound/WAV/AMB_LP_Phase3_V01.AMB_LP_Phase3_V01" 1.0 1.0 0.0 0))
      (Variables|Default|SetPhase3 _returnvalue_4))
    (:then_4
      (bind _returnvalue_5 (Audio|SpawnSound2D "/Game/Sound/WAV/AMB_LP_Phase4_V01.AMB_LP_Phase4_V01" 1.0 1.0 0.0 0))
      (Variables|Default|SetPhase4 _returnvalue_5))))

(event Collision|EventActorBeginOverlap
  (params (OtherActor :type Actor%20Object%20Reference)))

(event EventTick
  (params (DeltaSeconds :type Float%20%28single-precision%29))
  (bind _phase0 (Variables|Default|GetPhase0))
  (Utilities|FlowControl|Sequence
    (:then_0
      (if true
        (Audio|Components|Audio|AdjustVolume _phase0 0.0 0.0 "Linear" :!class /Script/Engine.AudioComponent)
        (else
          (Audio|Components|Audio|AdjustVolume _phase0 0.0 0.0 "Linear" :!class /Script/Engine.AudioComponent))))))

(fn ConstructionScript)