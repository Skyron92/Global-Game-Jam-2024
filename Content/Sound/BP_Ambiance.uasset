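; BP_Ambiance is an actor that starts the game's 2D ambience sounds.
; On BeginPlay it caches BP_FirstPersonGameMode, then spawns and stores the Phase 1 and Phase 4 sound cues.
; A crossfade driven by the game mode's PercentRef, fading Phase 1 down as Phase 4 rises, exists but is disconnected.
; Spawns for Phases 0, 2 and 3 are also unwired, and Tick is empty.
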(event EventBeginPlay
  (bind _asbp_first_person_game_mode (Utilities|Casting|CastToBP_FirstPersonGameMode (Game|GetGameMode)))
  (Variables|Default|SetGameModeRef _asbp_first_person_game_mode)
  (Utilities|FlowControl|Sequence
    (:then_1
      (bind _returnvalue (Audio|SpawnSound2D "/Game/Sound/SC/AMB/SC_Phase1.SC_Phase1" 1.0 1.0 0.0 0))
      (Variables|Default|SetPhase1 _returnvalue))
    (:then_4
      (bind _returnvalue_2 (Audio|SpawnSound2D "/Game/Sound/SC/AMB/SC_Phase4.SC_Phase4" 1.0 1.0 0.0 0))
      (Variables|Default|SetPhase4 _returnvalue_2))))

(event Collision|EventActorBeginOverlap
  (params (OtherActor :type Actor%20Object%20Reference)))

(event EventTick
  (params (DeltaSeconds :type Float%20%28single-precision%29)))

(fn ConstructionScript)