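; BP_ObjectParent is a parent object that registers hard impacts, feeding the score and an anger gauge that can end the game.
; CasseCollision overlaps with anything except itself or the player check the speed of Objet against a threshold.
; A fast hit writes weight-times-speed values to the game mode and disables further overlaps.
; It then updates and pauses the HUD gauge, opening the GameOver level if full.
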(event OnComponentBeginOverlap(CasseCollision)
  (params (OverlappedComponent :type Primitive%20Component%20Object%20Reference) (OtherActor :type Actor%20Object%20Reference) (OtherComp :type Primitive%20Component%20Object%20Reference) (OtherBodyIndex :type Integer) (bFromSweep :type Boolean) (SweepResult :type Hit%20Result%20Structure%20%28by%20ref%29))
  (bind _objet (Variables|Default|GetObjet))
  (bind _weight (Variables|Default|GetWeight))
  (bind _gamemoderef (Variables|Default|GetGameModeRef))
  (bind _returnvalue (Transformation|GetComponentVelocity _objet))
  (bind _returnvalue_2 (Math|Vector|VectorGetAbs _returnvalue))
  (bind _returnvalue_3 (Math|Vector|VectorLength _returnvalue_2))
  (bind _returnvalue_4 (* _weight _returnvalue_3))
  (if (!= OtherActor self)
    (Utilities|Casting|CastToBP_FirstPersonCharacter OtherActor
      (:CastFailed
        (Utilities|IsValid _gamemoderef
          (:Is%20Valid
            (Variables|Default|SetWBHudRefObjet (Variables|/Game/FirstPerson/Blueprints/BP_FirstPersonGameMode.BP_FirstPersonGameMode_C|GetWBHudRef _gamemoderef))
            (if (> _returnvalue_3 2e+02)
              (Variables|/Game/FirstPerson/Blueprints/BP_FirstPersonGameMode.BP_FirstPersonGameMode_C|SetScoreRef _gamemoderef _returnvalue_4)
              (Variables|/Game/FirstPerson/Blueprints/BP_FirstPersonGameMode.BP_FirstPersonGameMode_C|SetWeightRef (Variables|Default|GetGameModeRef) (Math|Float|Truncate (* _returnvalue_4 0.001)))
              (Variables|/Script/Engine.PrimitiveComponent|SetbGenerateOverlapEvents (Variables|Default|GetCasseCollision) false)
              (Default|AngryJauge (Variables|Default|GetWBHudRefObjet) 0.0)
              (Variables|/Game/Blueprint/Widget/WB_HUD.WB_HUD_C|SetJaugePause (Variables|Default|GetWBHudRefObjet) true)
              (if (>= (Variables|/Script/UMG.ProgressBar|GetPercent (Variables|/Game/Blueprint/Widget/WB_HUD.WB_HUD_C|GetProgressBar_0 (Variables|Default|GetWBHudRefObjet))) 1.0)
                (Game|OpenLevel(byObjectReference) "/Game/Maps/GameOver.GameOver")
                (Development|PrintString "game over")))))))))

(event EventBeginPlay
  (Utilities|FlowControl|Delay 1e-06)
  (bind _asbp_first_person_game_mode (Utilities|Casting|CastToBP_FirstPersonGameMode (Game|GetGameMode)))
  (Variables|Default|SetGameModeRef _asbp_first_person_game_mode))

(event Collision|EventActorBeginOverlap
  (params (OtherActor :type Actor%20Object%20Reference)))

(event EventTick
  (params (DeltaSeconds :type Float%20%28single-precision%29)))

(fn ConstructionScript)