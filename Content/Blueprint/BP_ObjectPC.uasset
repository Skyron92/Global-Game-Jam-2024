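; BP_ObjectPC is a PC object that changes appearance and loses its attached parts when hit.
; The construction script caches the direct children of the Objet component in PCParts.
; A hit on Objet by another actor swaps its second material slot to BackgroundMaterial and destroys those parts.
; The loop removes entries from PCParts while iterating it, so a single hit can skip some parts.
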(event OnComponentHit(Objet)
  (params (HitComponent :type Primitive%20Component%20Object%20Reference) (OtherActor :type Actor%20Object%20Reference) (OtherComp :type Primitive%20Component%20Object%20Reference) (NormalImpulse :type Vector :default "0, 0, 0") (Hit :type Hit%20Result%20Structure%20%28by%20ref%29))
  (bind _pc_parts (Variables|Default|GetPC_Parts))
  (if (!= OtherActor self)
    (Rendering|Material|SetMaterial (Variables|Default|GetObjet) 1 "/Engine/EngineMeshes/BackgroundMaterial.BackgroundMaterial")
    (for (_array_element _array_index) _pc_parts
      (Components|DestroyComponent _array_element)
      (Utilities|Array|RemoveItem _pc_parts (Utilities|Array|Get(acopy) _pc_parts _array_index)))))

(event EventBeginPlay
  (|CallParentFunction))

(event Collision|EventActorBeginOverlap
  (params (OtherActor :type Actor%20Object%20Reference))
  (|CallParentFunction OtherActor) ; This node is disabled and will not be called.\nDrag off pins to build functionality.
)

(event EventTick
  (params (DeltaSeconds :type Float%20%28single-precision%29))
  (|CallParentFunction DeltaSeconds) ; This node is disabled and will not be called.\nDrag off pins to build functionality.
)

(fn ConstructionScript
  (|CallParentFunction)
  (Variables|Default|SetPC_Parts (Components|GetChildrenComponents (Variables|Default|GetObjet) false)))