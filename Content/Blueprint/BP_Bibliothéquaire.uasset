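; Librarian NPC that watches for the player with a vision cone and turns its head periodically.
; Cone overlaps with the player set the HUD's Hidden flag on entry and clear it on exit, via the GameMode.
; MoveHead multiplies the mesh's yaw by a random factor in delay loops started at BeginPlay and each cone exit, with nothing stopping them.
; Tick switches the glass material to an angry version once the GameMode percentage reaches 60.
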(event OnComponentBeginOverlap(Cone)
  (params (OverlappedComponent :type Primitive%20Component%20Object%20Reference) (OtherActor :type Actor%20Object%20Reference) (OtherComp :type Primitive%20Component%20Object%20Reference) (OtherBodyIndex :type Integer) (bFromSweep :type Boolean) (SweepResult :type Hit%20Result%20Structure%20%28by%20ref%29))
  (Utilities|Casting|CastToBP_FirstPersonCharacter OtherActor)
  (Development|PrintString "La bibliothéquaire voit le joueur ")
  (Variables|/Game/Blueprint/Widget/WB_HUD.WB_HUD_C|SetHidden? (Variables|/Game/FirstPerson/Blueprints/BP_FirstPersonGameMode.BP_FirstPersonGameMode_C|GetWBHudRef (Variables|Default|GetGameModeRef)) true))

(event OnComponentEndOverlap(Cone)
  (params (OverlappedComponent :type Primitive%20Component%20Object%20Reference) (OtherActor :type Actor%20Object%20Reference) (OtherComp :type Primitive%20Component%20Object%20Reference) (OtherBodyIndex :type Integer))
  (Utilities|Casting|CastToBP_FirstPersonCharacter OtherActor)
  (Variables|/Game/Blueprint/Widget/WB_HUD.WB_HUD_C|SetHidden? (Variables|/Game/FirstPerson/Blueprints/BP_FirstPersonGameMode.BP_FirstPersonGameMode_C|GetWBHudRef (Variables|Default|GetGameModeRef)) false)
  (CallFunction|MoveHead :!label _label)
  (Utilities|FlowControl|Delay (Math|Random|RandomFloatinRange 2.0 6.0))
  (goto _label))

(event EventBeginPlay
  (bind _asbp_first_person_game_mode (Utilities|Casting|CastToBP_FirstPersonGameMode (Game|GetGameMode)))
  (Variables|Default|SetGameModeRef _asbp_first_person_game_mode)
  (if (not (Variables|/Game/Blueprint/Widget/WB_HUD.WB_HUD_C|GetHidden? (Variables|/Game/FirstPerson/Blueprints/BP_FirstPersonGameMode.BP_FirstPersonGameMode_C|GetWBHudRef (Variables|Default|GetGameModeRef))))
    (CallFunction|MoveHead :!label _label)
    (Utilities|FlowControl|Delay 6.0)
    (goto _label)))

(event Collision|EventActorBeginOverlap
  (params (OtherActor :type Actor%20Object%20Reference)))

(event EventTick
  (params (DeltaSeconds :type Float%20%28single-precision%29))
  (bind _skeletalmesh (Variables|Default|GetSkeletalMesh))
  (if (>= (* (Variables|/Game/FirstPerson/Blueprints/BP_FirstPersonGameMode.BP_FirstPersonGameMode_C|GetPercentRef (Variables|Default|GetGameModeRef)) 1e+02) 6e+01)
    (Rendering|Material|SetMaterial _skeletalmesh 6 "/Game/Assets/StaticMeshes/Bibliothécaire/angryGlass.angryGlass")
    (else
      (Rendering|Material|SetMaterial _skeletalmesh 6 "/Game/Assets/StaticMeshes/Bibliothécaire/glass.glass"))))

(fn ConstructionScript)

(fn MoveHead
  (params (FirstPersonReft :type BP%20First%20Person%20Character%20Object%20Reference))
  (bind _returnvalue (Math|Random|RandomFloatinRange 25.0 9e+01))
  (bind _staticmesh (Variables|Default|GetStaticMesh))
  (Development|PrintString (Utilities|String|ToString(Float) _returnvalue))
  (Transformation|SetWorldRotation _staticmesh (Math|Rotator|MakeRotator 0.0 0.0 (* (.yaw (Transformation|GetWorldRotation _staticmesh)) _returnvalue)) false false))